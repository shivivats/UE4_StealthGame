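; BP_LaunchPadTest is a launch pad that flings whatever overlaps its collision box.
; Each overlap spawns a particle burst at the other actor, then builds a velocity from the pad's horizontal forward direction and separate XY and Z force variables.
; An FPSCharacter gets LaunchCharacter with both overrides, while anything else receives a mass-independent velocity-change impulse on the overlapping component.
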(event `self.CollisionBox.OnComponentBeginOverlap`
  (params (OverlappedComponent :type "PrimitiveComponent Object Reference") (OtherActor :type "Actor Object Reference") (OtherComp :type "PrimitiveComponent Object Reference") (OtherBodyIndex :type Integer) (bFromSweep :type Boolean) (SweepResult :type "HitResult Structure (by ref)"))
  (bind _launchforcexy (`self.LaunchForceXY`))
  (bind _returnvalue (`KismetMathLibrary.MakeVector` (* (.x (`self.GetActorForwardVector`)) _launchforcexy) (* (.y (`self.GetActorForwardVector`)) _launchforcexy) (`self.LaunchForceZ`)))
  (`GameplayStatics.SpawnEmitterAtLocation` "/Game/Effects/P_gold_ore_appearance.P_gold_ore_appearance" (`self.K2_GetActorLocation` OtherActor) (struct) (2.0 2.0 2.0))
  (bind _asfpscharacter (cast `FPSCharacter` OtherActor)
    (:`then`
      (`Character.LaunchCharacter` _asfpscharacter _returnvalue true true))
    (:`CastFailed`
      (`PrimitiveComponent.AddImpulse` OtherComp _returnvalue "None" true))))

(fn `UserConstructionScript`)