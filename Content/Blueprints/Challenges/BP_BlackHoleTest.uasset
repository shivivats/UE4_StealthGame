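; BP_BlackHoleTest is a test black hole actor that pulls in and destroys cube actors.
; Each Tick, static mesh components overlapping AttractingSphere whose owner name contains "Cube" get a mass-independent force toward the center, scaled by distance and Force, so pull grows farther out.
; Matching owners overlapping DestroyingSphere are then destroyed.
; An AddRadialForce alternative remains unconnected.
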(event `self.ReceiveTick`
  (params (DeltaSeconds :type "Float (single-precision)"))
  (bind _returnvalue (`self.K2_GetActorLocation`))
  (`|ExecutionSequence`
    (:`then_0`
      (for _array_element (`PrimitiveComponent.GetOverlappingComponents` (`self.AttractingSphere`))
        (bind _asstatic_mesh_component (cast `StaticMeshComponent` _array_element))
        (bind _returnvalue_2 (`ActorComponent.GetOwner` _asstatic_mesh_component))
        (if (`KismetStringLibrary.Contains` (`KismetSystemLibrary.GetObjectName` _returnvalue_2) "Cube")
          (bind _returnvalue_3 (`self.K2_GetActorLocation` _returnvalue_2))
          (`PrimitiveComponent.AddForce` _asstatic_mesh_component (* (* (`KismetMathLibrary.Conv_RotatorToVector` (`KismetMathLibrary.FindLookAtRotation` _returnvalue_3 _returnvalue)) (`KismetMathLibrary.VSize` (- _returnvalue _returnvalue_3))) (`self.Force`)) "None" true))))
    (:`then_1`
      (for _array_element_2 (`PrimitiveComponent.GetOverlappingComponents` (`self.DestroyingSphere`))
        (bind _asstatic_mesh_component_2 (cast `StaticMeshComponent` _array_element_2))
        (bind _returnvalue_4 (`ActorComponent.GetOwner` _asstatic_mesh_component_2))
        (if (`KismetStringLibrary.Contains` (`KismetSystemLibrary.GetObjectName` _returnvalue_4) "Cube")
          (`self.K2_DestroyActor` _returnvalue_4))))))

(fn `UserConstructionScript`)